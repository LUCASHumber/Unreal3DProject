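; BP_TempSkeeBall is a trigger that starts skee-ball play when the player character walks into it.
; On Box overlap by the player character, it finds the BP_SkeeBall actor in the level and has the player controller possess it.
; It then creates a PowerBoxText widget and adds it to the viewport.
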(event OnComponentBeginOverlap(Box)
  (params (OverlappedComponent :type Primitive%20Component%20Object%20Reference) (OtherActor :type Actor%20Object%20Reference) (OtherComp :type Primitive%20Component%20Object%20Reference) (OtherBodyIndex :type Integer) (bFromSweep :type Boolean) (SweepResult :type Hit%20Result%20Structure%20%28by%20ref%29))
  (if (== OtherActor (Game|GetPlayerCharacter 0))
    (bind _returnvalue (Actor|GetActorOfClass "/Game/MyBlueprints/BP_SkeeBall.BP_SkeeBall_C"))
    (Variables|Default|SetTemo _returnvalue)
    (Pawn|Possess (Game|GetPlayerController 0) (Variables|Default|GetTemo))
    (bind _returnvalue_2 (UserInterface|CreateWidget "/Game/InterfaceWidgets/PowerBoxText.PowerBoxText_C"))
    (bind _output_get (Variables|Default|Setis%20Ball%20View _returnvalue_2))
    (UserInterface|Viewport|AddtoViewport _output_get 0)))

(event EventBeginPlay)

(event Collision|EventActorBeginOverlap
  (params (OtherActor :type Actor%20Object%20Reference)))

(event EventTick
  (params (DeltaSeconds :type Float%20%28single-precision%29)))

(fn ConstructionScript)